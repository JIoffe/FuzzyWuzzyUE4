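; BP_PlasmaBolt is a plasma projectile that damages the actor it hits.
; Tick moves it forward at a fixed speed with an unswept world offset.
; Overlapping any actor except its owner applies fixed damage if that actor can be damaged, credited to the owner's instigator controller.
; It then spawns an impact emitter and destroys itself, whether or not damage was applied.
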(event `self.ReceiveTick`
  (params (DeltaSeconds :type "Float (single-precision)"))
  (`self.K2_AddActorWorldOffset` (* (`self.GetActorForwardVector`) (* DeltaSeconds 2000.0))))

(event `self.ReceiveActorBeginOverlap`
  (params (OtherActor :type "Actor Object Reference"))
  (bind _returnvalue (`self.GetOwner`))
  (if (!= OtherActor _returnvalue)
    (`|ExecutionSequence`
      (:`then_0`
        (if (`Actor.bCanBeDamaged` OtherActor)
          (`GameplayStatics.ApplyDamage` OtherActor 40.0 (`self.GetInstigatorController` _returnvalue) self)))
      (:`then_1`
        (`GameplayStatics.SpawnEmitterAtLocation` "/Game/FX/PS_PlasmaBoltImpact.PS_PlasmaBoltImpact" (`self.K2_GetActorLocation`))
        (`self.K2_DestroyActor`)))))

(fn `UserConstructionScript`)