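; BP_SimpleAgroCharacter is an AI enemy that turns on whoever damages it and dissolves when killed.
; Damage reveals a screen-space health widget, refreshed each tick, and writes the instigator to the blackboard as PlayerActor.
; At zero health it stops AI logic, disables collision and drives a dissolve material parameter until destroyed after a delay.
; ToggleHitbox switches the attack hitbox's query collision on or off.
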(event `self.ReceiveBeginPlay`
  (bind _enemystatus (`self.EnemyStatus`))
  (bind _mesh (`self.Mesh`))
  (set `self.MaxHealth` (`self.Health`))
  (bind _returnvalue (`PrimitiveComponent.CreateDynamicMaterialInstance` _mesh 0 (`PrimitiveComponent.GetMaterial` _mesh 0) "None"))
  (set `self.DissolveMaterialInstance` _returnvalue)
  (`WidgetComponent.SetWidgetSpace` _enemystatus "Screen")
  (`SceneComponent.SetHiddenInGame` _enemystatus true false))

(event `self.ReceiveTick`
  (params (DeltaSeconds :type "Float (single-precision)"))
  (`self.UpdateHealthDisplay`)
  (if (<= (`self.Health`) 0.0)
    (bind _output_get (set `self.DissolveAmount` (+ (* DeltaSeconds (`self.DissolveRate`)) (`self.DissolveAmount`))))
    (`MaterialInstanceDynamic.SetScalarParameterValue` (`self.DissolveMaterialInstance`) "DissolveAmount" (`KismetMathLibrary.FClamp` _output_get))))

(event `self.ReceiveAnyDamage`
  (params (Damage :type "Float (single-precision)") (DamageType :type "DamageType Object Reference") (InstigatedBy :type "Controller Object Reference") (DamageCauser :type "Actor Object Reference"))
  (`SceneComponent.SetHiddenInGame` (`self.EnemyStatus`) false true)
  (bind _output_get (set `self.Health` (- (`self.Health`) Damage)))
  (if (<= _output_get 0.0)
    ;[1 1 1] Death
    (`BrainComponent.StopLogic` (`AIController.BrainComponent` (`AIBlueprintHelperLibrary.GetAIController` self)) "")
    (`self.SetActorEnableCollision` false)
    (`KismetSystemLibrary.Delay` (`self.PersistTimeAfterDeath`))
    (`self.K2_DestroyActor`)
    (else
      ;[1 1 1] Psst. Attack the player.
      (`BlackboardComponent.SetValueAsObject` (`AIBlueprintHelperLibrary.GetBlackboard` (`AIBlueprintHelperLibrary.GetAIController` self)) "PlayerActor" InstigatedBy))))

(fn `Toggle Hitbox`
  (params (ShouldCollide :type Boolean))
  (bind _attackhitbox (`self.AttackHitbox`))
  (if ShouldCollide
    (`PrimitiveComponent.SetCollisionEnabled` _attackhitbox "QueryOnly")
    (else
      (`PrimitiveComponent.SetCollisionEnabled` _attackhitbox "NoCollision"))))

(fn `UpdateHealthDisplay`
  (bind _asbp_enemy_health (cast `/Game/Characters/Baddies/BP_EnemyHealth` (`WidgetComponent.GetWidget` (`self.EnemyStatus`))))
  (`/Game/Characters/Baddies/BP_EnemyHealth.HealthUpdated` _asbp_enemy_health (`self.Health`) (`self.MaxHealth`)))

(fn `UserConstructionScript`)